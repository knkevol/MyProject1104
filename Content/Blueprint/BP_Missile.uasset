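; BP_Missile is a short-lived missile actor that destroys actors tagged "Target" when it overlaps them.
; BeginPlay sets a life span so the missile removes itself after a few seconds.
; On a hit it destroys the target, spawns an explosion particle, calls CustomEvent on BP_GM, then destroys itself.
; The explosion sound node is left unconnected, so it never plays.
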(event EventBeginPlay
  ;[0.15 0.15 0.15 0.5 15] Delay + Destroy Actor
  (Actor|SetLifeSpan 3.0))

(event Collision|EventActorBeginOverlap
  (params (OtherActor :type Actor%20Object%20Reference))
  (if (Actor|ActorHasTag OtherActor "Target")
    ;[0.15 0.15 0.15 0.5] Sphere Destroy
    (Actor|DestroyActor OtherActor)
    (Effects|SpawnEmitteratLocation "/Game/StarterContent/Particles/P_Explosion.P_Explosion" (Transformation|GetActorLocation))
    (bind _asbp_gm (Utilities|Casting|CastToBP_GM (Game|GetGameMode)))
    (Default|CustomEvent _asbp_gm)
    ;[0.15 0.15 0.15 0.5] Particle Destroy
    (Actor|DestroyActor)))

(fn ConstructionScript)