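; BP_P38 is a player-controlled P-38 aircraft pawn that constantly flies forward.
; Tick feeds full forward movement input and spins the Left and Right components on their roll axis at RotateSpeed.
; Pitch and Roll axes apply frame-rate-independent local rotation to the actor, while Fire only prints a debug message.
; A MoveForward function offers offset-based movement but is not called in this graph.
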(event EventTick
  (params (DeltaSeconds :type Float%20%28single-precision%29))
  ;[0.15 0.15 0.15 0.5 13] ScaleValue : 속력조절가능
  (Pawn|Input|AddMovementInput (Transformation|GetActorForwardVector) 1.0 false)
  (CallFunction|RotateComponent (Variables|Default|GetLeft))
  (CallFunction|RotateComponent (Variables|Default|GetRight)))

(event Input|ActionEvents|InputActionFire
  (params (Key :type Key%20Structure :default "None"))
  (:Pressed
    (Development|PrintString "Shoot")))

(event Input|AxisEvents|InputAxisPitch
  (params (AxisValue :type Float%20%28single-precision%29))
  (Transformation|AddActorLocalRotation (Math|Rotator|MakeRotator 0.0 (* AxisValue (Utilities|Time|GetWorldDeltaSeconds) 45.0) 0.0) false false))

(event Input|AxisEvents|InputAxisRoll
  (params (AxisValue :type Float%20%28single-precision%29))
  (Transformation|AddActorLocalRotation (Math|Rotator|MakeRotator (* AxisValue (Utilities|Time|GetWorldDeltaSeconds) 45.0) 0.0 0.0) false false))

(fn ConstructionScript)

(fn MoveForward
  (params (Speed :type Float%20%28single-precision%29))
  (Transformation|AddActorWorldOffset (* (Transformation|GetActorForwardVector) Speed (Utilities|Time|GetWorldDeltaSeconds))))

(fn RotateComponent
  (params (Where :type Scene%20Component%20Object%20Reference))
  (Transformation|AddLocalRotation Where (Math|Rotator|MakeRotator (* (Utilities|Time|GetWorldDeltaSeconds) (Variables|Default|GetRotateSpeed)) 0.0 0.0) false false))